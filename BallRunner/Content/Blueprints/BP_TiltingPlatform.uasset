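; BP_TiltingPlatform is a platform that tilts once the player's BP_Ball enters its TriggerZone.
; The overlap sets IsTilting only when the overlapping actor is that player pawn, and nothing in this graph clears it.
; Tick interpolates PlatformMesh roll toward TiltAngle at TiltSpeed while tilting, otherwise toward level, with delta time scaled down to slow the motion.
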(event `self.TriggerZone.OnComponentBeginOverlap`
  (params (OverlappedComponent :type "PrimitiveComponent Object Reference") (OtherActor :type "Actor Object Reference") (OtherComp :type "PrimitiveComponent Object Reference") (OtherBodyIndex :type Integer) (bFromSweep :type Boolean) (SweepResult :type "HitResult Structure (by ref)"))
  (bind _asbp_ball (cast `/Game/Blueprints/BP_Ball` (`GameplayStatics.GetPlayerPawn` 0)))
  (if (== _asbp_ball OtherActor)
    (set `self.IsTilting` true)))

(event `self.ReceiveTick`
  (params (DeltaSeconds :type "Float (single-precision)"))
  (bind _returnvalue (* DeltaSeconds 0.1))
  (bind _tiltspeed (`self.TiltSpeed`))
  (bind _platformmesh (`self.PlatformMesh`))
  (bind _relativerotation_roll (`KismetMathLibrary.BreakRotator` (`SceneComponent.RelativeRotation` _platformmesh)))
  (if (`self.IsTilting`)
    (`SceneComponent.K2_SetRelativeRotation` _platformmesh (`KismetMathLibrary.MakeRotator` (`KismetMathLibrary.FInterpTo` _relativerotation_roll (`self.TiltAngle`) _returnvalue _tiltspeed)) false false)
    (else
      (`SceneComponent.K2_SetRelativeRotation` _platformmesh (`KismetMathLibrary.MakeRotator` (`KismetMathLibrary.FInterpTo` _relativerotation_roll 0.0 _returnvalue _tiltspeed)) false false))))

(fn `UserConstructionScript`)